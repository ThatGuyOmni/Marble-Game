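; BP_BallCharacter is the player character, a ball that moves relative to camera yaw, jumps, and heads for a BP_EndLevel actor.
; Enhanced Input drives character movement, while BallBody is spun at a fixed rate regardless of input sign to fake rolling.
; BeginPlay creates the HUD and starts a looping timer updating the yaw toward the level end.
; It also handles Escape-to-quit and a pausing win screen; look-input nodes are unwired.
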(event Custom|ActivateUI
  ;[0 0.5549 1] UI
  (bind _returnvalue (UserInterface|CreateWidget "/Game/Project/Blueprints/UI/WBP_PlayerHud.WBP_PlayerHud_C"))
  (bind _output_get (Variables|Default|SetHud _returnvalue))
  (UserInterface|Viewport|AddtoViewport _output_get 0)
  (Default|ActivateHud (Variables|Default|GetHud) self))

(event Custom|EndScreen
  ;[0 0.5549 1] UI
  (bind _returnvalue (UserInterface|CreateWidget "/Game/Project/Blueprints/UI/WBP_WinScreen.WBP_WinScreen_C"))
  (UserInterface|Viewport|AddtoViewport _returnvalue 0)
  (Game|SetGamePaused true))

(event Custom|Waypoint
  (Variables|Default|SetWaypointLocation (.yaw (Math|Rotator|FindLookatRotation (Transformation|GetActorLocation) (Variables|Default|GetEndLevelLocation)))))

(event Input|EnhancedActionEvents|EnhancedInputActionIA_Jump
  (params (ActionValue :type Boolean) (ElapsedSeconds :type Float%20%28double-precision%29) (TriggeredSeconds :type Float%20%28double-precision%29) (InputAction :type Input%20Action%20Object%20Reference :default "/Game/Project/Controller/Inputs/IA_Jump.IA_Jump"))
  ;[0 1 0.01606] Controls
  (:Triggered
    (Character|Jump))
  (:Completed
    (Character|StopJumping)))

(event Input|EnhancedActionEvents|EnhancedInputActionIA_MoveSides
  (params (ActionValue :type Float%20%28double-precision%29) (ElapsedSeconds :type Float%20%28double-precision%29) (TriggeredSeconds :type Float%20%28double-precision%29) (InputAction :type Input%20Action%20Object%20Reference :default "/Game/Project/Controller/Inputs/IA_MoveSides.IA_MoveSides"))
  ;[0 1 0.01606] Controls
  (:Triggered
    (Pawn|Input|AddMovementInput (Math|Vector|GetRightVector (Math|Rotator|MakeRotator 0.0 0.0 (.yaw (Pawn|GetControlRotation :!class /Script/Engine.Pawn)))) ActionValue false)
    (bind _output_get (Variables|Default|SetCurrentSpeed 2e+02))
    (Variables|Default|SetRotationSpeed (* _output_get -0.02))
    (Transformation|AddLocalRotation (Variables|Default|GetBallBody) (Math|Rotator|MakeRotator (Variables|Default|GetRotationSpeed) 0.0 0.0) false false))
  (:Completed
    (Variables|Default|SetCurrentSpeed 0.0)))

(event Input|EnhancedActionEvents|EnhancedInputActionIA_MoveForward
  (params (ActionValue :type Float%20%28double-precision%29) (ElapsedSeconds :type Float%20%28double-precision%29) (TriggeredSeconds :type Float%20%28double-precision%29) (InputAction :type Input%20Action%20Object%20Reference :default "/Game/Project/Controller/Inputs/IA_MoveForward.IA_MoveForward"))
  ;[0 1 0.01606] Controls
  (:Triggered
    (Pawn|Input|AddMovementInput (Math|Vector|GetForwardVector (Math|Rotator|MakeRotator 0.0 0.0 (.yaw (Pawn|GetControlRotation :!class /Script/Engine.Pawn)))) ActionValue false)
    (bind _output_get (Variables|Default|SetCurrentSpeed 2e+02))
    (Variables|Default|SetRotationSpeed (* _output_get -0.02))
    (Transformation|AddLocalRotation (Variables|Default|GetBallBody) (Math|Rotator|MakeRotator 0.0 (Variables|Default|GetRotationSpeed) 0.0) false false))
  (:Completed
    (Variables|Default|SetCurrentSpeed 0.0)))

(event Input|EnhancedActionEvents|EnhancedInputActionIA_Look
  (params (ActionValue :type Vector%202D%20Structure) (ElapsedSeconds :type Float%20%28double-precision%29) (TriggeredSeconds :type Float%20%28double-precision%29) (InputAction :type Input%20Action%20Object%20Reference :default "/Game/Project/Controller/Inputs/IA_Look.IA_Look"))
  ;[0 1 0.01606] Controls
)

(event EventBeginPlay
  ;[0 0.5549 1] UI
  (CallFunction|ActivateUI)
  (bind _returnvalue (Actor|GetActorOfClass "/Game/Project/Blueprints/BP_EndLevel.BP_EndLevel_C"))
  (Variables|Default|SetEndLevelLocation (Transformation|GetActorLocation _returnvalue))
  (Utilities|Time|SetTimerbyEvent (delegate Custom|Waypoint) 0.01 true))

(event Input|KeyboardEvents|Escape
  (params (Key :type Key%20Structure :default "None"))
  (:Pressed
    (Game|QuitGame 0 "Quit" true)))

(fn ConstructionScript)