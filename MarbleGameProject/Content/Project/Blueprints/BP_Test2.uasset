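; BP_Test2 is an input test Blueprint that rotates its Plane component with Enhanced Input.
; While triggered, IA_MoveForward applies local pitch and IA_MoveSides local roll, using a fixed step derived from a hardcoded CurrentSpeed.
; The step ignores input value and delta time, so each axis turns one way at a trigger-rate-dependent speed.
; Releasing either action zeroes CurrentSpeed; forward input also prints a debug string.
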(event Input|EnhancedActionEvents|EnhancedInputActionIA_MoveSides
  (params (ActionValue :type Float%20%28double-precision%29) (ElapsedSeconds :type Float%20%28double-precision%29) (TriggeredSeconds :type Float%20%28double-precision%29) (InputAction :type Input%20Action%20Object%20Reference :default "/Game/Project/Controller/Inputs/IA_MoveSides.IA_MoveSides"))
  (:Triggered
    (bind _output_get (Variables|Default|SetCurrent%20Speed 2e+02))
    (Variables|Default|SetRotaion%20Speed (* _output_get -0.02))
    (Transformation|AddLocalRotation (Variables|Default|GetPlane) (Math|Rotator|MakeRotator (Variables|Default|GetRotaion%20Speed) 0.0 0.0) false false))
  (:Completed
    (Variables|Default|SetCurrent%20Speed 0.0)))

(event Input|EnhancedActionEvents|EnhancedInputActionIA_MoveForward
  (params (ActionValue :type Float%20%28double-precision%29) (ElapsedSeconds :type Float%20%28double-precision%29) (TriggeredSeconds :type Float%20%28double-precision%29) (InputAction :type Input%20Action%20Object%20Reference :default "/Game/Project/Controller/Inputs/IA_MoveForward.IA_MoveForward"))
  (:Triggered
    (Development|PrintString "Hello")
    (bind _output_get (Variables|Default|SetCurrent%20Speed 2e+02))
    (Variables|Default|SetRotaion%20Speed (* _output_get -0.02))
    (Transformation|AddLocalRotation (Variables|Default|GetPlane) (Math|Rotator|MakeRotator 0.0 (Variables|Default|GetRotaion%20Speed) 0.0) false false))
  (:Completed
    (Variables|Default|SetCurrent%20Speed 0.0)))

(fn ConstructionScript)