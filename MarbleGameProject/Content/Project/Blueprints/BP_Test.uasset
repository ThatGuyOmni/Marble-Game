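; BP_Test is a test character Blueprint that spins a BallBody component from Enhanced Input, with jump and an Escape key that quits the game.
; Forward and sideways actions set a fixed CurrentSpeed, derive RotationSpeed from it, and add local pitch or roll per trigger, ignoring input sign.
; Releasing either action zeroes CurrentSpeed.
; No movement input is applied here, and the camera look nodes are disconnected.
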(event Input|EnhancedActionEvents|EnhancedInputActionIA_Jump
  (params (ActionValue :type Boolean) (ElapsedSeconds :type Float%20%28double-precision%29) (TriggeredSeconds :type Float%20%28double-precision%29) (InputAction :type Input%20Action%20Object%20Reference :default "/Game/Project/Controller/Inputs/IA_Jump.IA_Jump"))
  ;[0 1 0.01606] Controls
  (:Triggered
    (Character|Jump))
  (:Completed
    (Character|StopJumping)))

(event Input|EnhancedActionEvents|EnhancedInputActionIA_MoveSides
  (params (ActionValue :type Float%20%28double-precision%29) (ElapsedSeconds :type Float%20%28double-precision%29) (TriggeredSeconds :type Float%20%28double-precision%29) (InputAction :type Input%20Action%20Object%20Reference :default "/Game/Project/Controller/Inputs/IA_MoveSides.IA_MoveSides"))
  ;[0 1 0.01606] Controls
  (:Triggered
    (bind _output_get (Variables|Default|SetCurrentSpeed 2e+02))
    (Variables|Default|SetRotationSpeed (* _output_get -0.02))
    (Transformation|AddLocalRotation (Variables|Default|GetBallBody) (Math|Rotator|MakeRotator (Variables|Default|GetRotationSpeed) 0.0 0.0) false false))
  (:Completed
    (Variables|Default|SetCurrentSpeed 0.0)))

(event Input|EnhancedActionEvents|EnhancedInputActionIA_MoveForward
  (params (ActionValue :type Float%20%28double-precision%29) (ElapsedSeconds :type Float%20%28double-precision%29) (TriggeredSeconds :type Float%20%28double-precision%29) (InputAction :type Input%20Action%20Object%20Reference :default "/Game/Project/Controller/Inputs/IA_MoveForward.IA_MoveForward"))
  ;[0 1 0.01606] Controls
  (:Triggered
    (bind _output_get (Variables|Default|SetCurrentSpeed 2e+02))
    (Variables|Default|SetRotationSpeed (* _output_get -0.02))
    (Transformation|AddLocalRotation (Variables|Default|GetBallBody) (Math|Rotator|MakeRotator 0.0 (Variables|Default|GetRotationSpeed) 0.0) false false))
  (:Completed
    (Variables|Default|SetCurrentSpeed 0.0)))

(event Input|EnhancedActionEvents|EnhancedInputActionIA_Look
  (params (ActionValue :type Vector%202D%20Structure) (ElapsedSeconds :type Float%20%28double-precision%29) (TriggeredSeconds :type Float%20%28double-precision%29) (InputAction :type Input%20Action%20Object%20Reference :default "/Game/Project/Controller/Inputs/IA_Look.IA_Look"))
  ;[0 1 0.01606] Controls
)

(event Input|KeyboardEvents|Escape
  (params (Key :type Key%20Structure))
  (:Pressed
    (Game|QuitGame 0 "Quit" false)))

(fn ConstructionScript)