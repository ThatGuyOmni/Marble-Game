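; Actor that bridges the game to an Arduino over a serial COM port, opened on BeginPlay and closed on EndPlay or Destroyed.
; Each tick it reads a line, prints it, parses comma-separated key/value pairs into a string map and broadcasts DataReceived, then requests input pins again.
; SendData writes arbitrary strings to the port.
; A P debug key prints "Hello World!" as ASCII codes.
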(event Custom|Init
  ;[0 1 0.1111 0.25] Open Port
  (bind (_bopened _returnvalue) (Class|SerialCom|OpenComPortwithFlowControl (Variables|Default|GetPort) 9600 true true))
  (if _bopened
    (bind _output_get (Variables|Default|SetSerialCOM _returnvalue))
    (Class|SerialCom|Flush _output_get)
    (else
      (Development|PrintString "Port Failure!" true true "(R=0.000000,G=0.660000,B=1.000000,A=1.000000)" 2e+01))))

(event Custom|PrintCharacters
  (bind _returnvalue (Utilities|String|MakeLiteralString "Hello World!"))
  ;[1 1 1 0.25] ASCII Demo
  (for _index (range 0 (Utilities|String|Len _returnvalue))
    (Development|PrintString (Utilities|String|ToString(Integer) (Utilities|String|GetCharacterasNumber _returnvalue _index)))))

(event Custom|ReadData
  ;[0 1 0.3514 0.25] Read Arduino Data
  (bind _serialcom (Variables|Default|GetSerialCOM)
    (:then
      (bind (_bsuccess _returnvalue) (Class|SerialCom|Readln _serialcom))
      (if _bsuccess
        (Development|PrintString _returnvalue true false "(R=0.000000,G=1.000000,B=0.042082,A=1.000000)" 2.0 "AnalogData")
        (CallFunction|ParseData _returnvalue)
        (Default|CallDataReceived _returnvalue (Variables|Default|GetStringMap))))
    (:else)))

(event Custom|ParseData
  (params (IncomingSerialData :type String))
  ;[1 0.9231 0 0.25] Parse Arduino Data
  (for _array_element (Utilities|String|ParseIntoArray IncomingSerialData ",")
    (Utilities|Map|Add (Variables|Default|GetStringMap) (.Key (Class|GameplayStatics|GetKeyValue _array_element)) (.Value (Class|GameplayStatics|GetKeyValue _array_element)))))

(event Custom|RequestInputPins
  (bind _serialcom (Variables|Default|GetSerialCOM)
    (:then
      (bind _returnvalue (Class|SerialCom|Println _serialcom "ReadPins=1"))
      (if (not _returnvalue)
        (Development|PrintString "Error Sending Data to Arduino!")))
    (:else)))

(event Custom|SendData
  (params (DataString :type String))
  (bind _serialcom (Variables|Default|GetSerialCOM)
    (:then
      (bind _returnvalue (Class|SerialCom|Println _serialcom DataString))
      (if (not _returnvalue)
        (Development|PrintString "Error Sending Data to Arduino!")))
    (:else)))

(event EventBeginPlay
  ;[0 1 0.1111 0.25] Open Port
  (CallFunction|Init))

(event EventEndPlay
  (params (EndPlayReason :type EEndPlayReason%20Enum :default "Destroyed"))
  ;[1 0 0.01201 0.25] Close Port
  (bind _serialcom (Variables|Default|GetSerialCOM)
    (:then
      (if (Class|SerialCom|IsOpened _serialcom)
        (Class|SerialCom|Close _serialcom)))
    (:else)))

(event EventDestroyed
  ;[1 0 0.01201 0.25] Close Port
  (bind _serialcom (Variables|Default|GetSerialCOM)
    (:then
      (if (Class|SerialCom|IsOpened _serialcom)
        (Class|SerialCom|Close _serialcom)))
    (:else)))

(event EventTick
  (params (DeltaSeconds :type Float%20%28single-precision%29))
  ;[0 1 0.3514 0.25] Read Arduino Data
  (CallFunction|ReadData)
  (CallFunction|RequestInputPins))

(event Input|KeyboardEvents|DebugKeyP
  (params (Key :type Key%20Structure :default "None") (ActionValue :type Input%20Action%20Value%20Structure))
  ;[1 1 1 0.25] ASCII Demo
  (:Pressed
    (CallFunction|PrintCharacters)))

(fn ConstructionScript)